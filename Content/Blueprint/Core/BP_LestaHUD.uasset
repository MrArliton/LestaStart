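; HUD for the Lesta character that creates the player UI widget and shows health and ammo.
; BeginPlay uses setup macros to find the owning pawn and build the widget, then binds health changes to it and removes it when the character is destroyed.
; Tick polls the current weapon's first BaseWeaponComponent, pushing max ammo to the widget and assigning the ammo-change binding every frame.
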(event `self.ReceiveBeginPlay`
  (bind _lesta_character (`self.Lesta Character`))
  ;[1 1 1] Construct Widgets
  (bind (_lesta_character_2 _living_attribute_component) (`self.Setup Lesta Character`)
    (:`Successful`
      (bind _player_ui_widget (`self.Setup UI Player Widget` (`self.GetOwningPlayerController`) "/Game/Blueprint/UI/BP_PlayerUIWidget.BP_PlayerUIWidget_C" _living_attribute_component)
        (:`End`
          (add `LivingAttributeComponent.OnChangeHealth` _living_attribute_component (delegate `OnChangeHealth_Event`))
          (`UserWidget.AddToViewport` _player_ui_widget 0)
          (if (`KismetSystemLibrary.IsValid` _lesta_character)
            (add `self.OnDestroyed` _lesta_character (delegate `OnDestroyed_Event`))))))
    (:`Unsuccessful`
      (`KismetSystemLibrary.PrintString` "Error with setup Lesta Character in HUD" false))))

(event `OnDestroyed_Event` :!signature `self.OnDestroyed`
  (params (DestroyedActor :type "Actor Object Reference"))
  ;[1 1 1] Construct Widgets
  (`Widget.RemoveFromParent` (`self.Player UI Widget`)))

(event `OnChangeHealth_Event`
  (params (Health :type "Float (single-precision)"))
  ;[1 1 1] Construct Widgets
  (`PlayerUIWidget.OnHealthChanged` (stale `self.ReceiveBeginPlay` _player_ui_widget) Health))

(event `self.ReceiveTick`
  (params (DeltaSeconds :type "Float (single-precision)"))
  (bind _lesta_character (`self.Lesta Character`))
  ;[1 1 1] Find weapons and bind
  (if (`KismetSystemLibrary.IsValid` _lesta_character)
    (bind _returnvalue (`LestaCharacter.GetCurrentWeaponActor` _lesta_character))
    (bind _output (`|GetArrayItem` (`self.K2_GetComponentsByClass` _returnvalue "/Script/LestaStart.BaseWeaponComponent")))
    (if (`KismetSystemLibrary.IsValid` _output)
      (bind _returnvalue_2 (`BaseWeaponComponent.GetMaxAmmo` _output))
      (`PlayerUIWidget.SetMaxAmmo` (`self.Player UI Widget`) _returnvalue_2)
      (add `BaseWeaponComponent.OnChangeAmmo` _output (delegate `OnChangeAmmo_Event`)))))

(event `OnChangeAmmo_Event`
  (params (Ammo :type "Float (single-precision)"))
  ;[1 1 1] Find weapons and bind
  (`PlayerUIWidget.OnAmmoChanged` (`self.Player UI Widget`) Ammo))

(fn `UserConstructionScript`)